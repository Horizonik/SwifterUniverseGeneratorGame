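; Camera controller that moves the player pawn along world X and Y axes from Enhanced Input.
; BeginPlay adds the input mapping context, then forward and right actions offset the pawn's location directly, without sweep.
; Both scale input by GetFrameIndependentSpeed, whose graph holds only an unconnected MovementSpeed-times-delta-time calculation.
; NormalizeSpeed offers similar delta-time scaling but is not called in these graphs.
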(event Input|EnhancedActionEvents|EnhancedInputActionIA_MoveForward
  (params (ActionValue :type Float%20%28double-precision%29) (ElapsedSeconds :type Float%20%28double-precision%29) (TriggeredSeconds :type Float%20%28double-precision%29) (InputAction :type Input%20Action%20Object%20Reference :default "/Game/Movement/Input/IA_MoveForward.IA_MoveForward"))
  (bind _returnvalue (Game|Player|GetPlayerPawn 0))
  ;[0 0 0] Forward / Backward movement
  (:Triggered
    (Transformation|SetActorLocation _returnvalue (+ (Transformation|GetActorLocation _returnvalue) (Math|Vector|MakeVector (.x (* ActionValue (Utilities|GetFrameIndependentSpeed))) 0.0 0.0)) false false)))

(event Input|EnhancedActionEvents|EnhancedInputActionIA_MoveRight
  (params (ActionValue :type Float%20%28double-precision%29) (ElapsedSeconds :type Float%20%28double-precision%29) (TriggeredSeconds :type Float%20%28double-precision%29) (InputAction :type Input%20Action%20Object%20Reference :default "/Game/Movement/Input/IA_MoveRight.IA_MoveRight"))
  (bind _returnvalue (Game|Player|GetPlayerPawn 0))
  ;[0 0 0] Right / Left movement
  (:Triggered
    (Transformation|SetActorLocation _returnvalue (+ (Transformation|GetActorLocation _returnvalue) (Math|Vector|MakeVector 0.0 (.y (* ActionValue (Utilities|GetFrameIndependentSpeed))) 0.0)) false false)))

(event EventBeginPlay
  (bind _returnvalue (PlayerController|LocalPlayerSubsystems|GetEnhancedInputLocalPlayerSubsystem))
  ;[0 0 0] Enable enhanced input
  (Utilities|IsValid _returnvalue
    (:Is%20Valid
      (Input|AddMappingContext _returnvalue "/Game/Movement/Input/IMC_InputMapping.IMC_InputMapping" 0 "(bIgnoreAllPressedKeysUntilRelease=True,bForceImmediately=False)"))))

(fn ConstructionScript)

(fn NormalizeSpeed
  (params (Speed :type Float%20%28double-precision%29))
  (return (* Speed (Utilities|Time|GetWorldDeltaSeconds))))