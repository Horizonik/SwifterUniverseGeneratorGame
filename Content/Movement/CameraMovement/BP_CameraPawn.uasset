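; BP_CameraPawn is a camera pawn with a spring arm.
; On BeginPlay it adds the IMC_InputMapping context to the Enhanced Input local player subsystem, when that subsystem is valid.
; It also holds zoom logic that lengthens or shortens the spring arm by ZoomAmount based on an action value, but no event triggers it, so it never runs.
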(event Input|EnhancedActionEvents|EnhancedInputActionIA_ScrollZoom
  (params (ActionValue :type Boolean) (ElapsedSeconds :type Float%20%28double-precision%29) (TriggeredSeconds :type Float%20%28double-precision%29) (InputAction :type Input%20Action%20Object%20Reference :default "/Game/Movement/Input/IA_ScrollZoom.IA_ScrollZoom")))

(event EventBeginPlay
  (bind _returnvalue (PlayerController|LocalPlayerSubsystems|GetEnhancedInputLocalPlayerSubsystem))
  ;[0 0 0] Enable enhanced input
  (Utilities|IsValid _returnvalue
    (:Is%20Valid
      (Input|AddMappingContext _returnvalue "/Game/Movement/Input/IMC_InputMapping.IMC_InputMapping" 0 "(bIgnoreAllPressedKeysUntilRelease=True,bForceImmediately=False)"))))

(fn ConstructionScript)